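; Test car Blueprint that prototypes raycast suspension on a physics Cube component.
; Each Tick it runs a debug-drawn object line trace from a point offset along world X from the Cube, along the Cube's up vector scaled by SuspensionRaycastDist.
; The trace result is unused, so no suspension force is applied yet.
; Space Bar applies a one-off upward local force at an offset location on the Cube.
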(event `self.ReceiveTick`
  (params (DeltaSeconds :type "Float (single-precision)"))
  (bind _cube (`self.Cube`))
  (bind _returnvalue (+ (`SceneComponent.K2_GetComponentLocation` _cube) (40.0 0.0 0.0)))
  (`KismetSystemLibrary.LineTraceSingleForObjects` :`Start` _returnvalue :`End` (+ _returnvalue (* (`KismetMathLibrary.GetUpVector` (`SceneComponent.K2_GetComponentRotation` _cube)) (`self.SuspensionRaycastDist`) 1.0)) :`ObjectTypes` (`self.Object Types`) :`DrawDebugType` "ForOneFrame"))

(event `Key|SpaceBar`
  (params (Key :type "Key Structure"))
  (:`Pressed`
    (`PrimitiveComponent.AddForceAtLocationLocal` (`self.Cube`) (0.0 0.0 25000.0) (1.0 1.0 0.0) "None")))

(fn `UserConstructionScript`)