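; Player-driven prototype car that accelerates, turns, strafes, drifts and boosts through input flags evaluated every Tick.
; Movement adds linear velocity to the physics body below speed caps, with yaw rotation only while a downward trace finds ground.
; Drifting ramps turn force and builds CurrentRad, which Boost spends for a higher top speed.
; Camera FOV widens with speed, and the spring arm swings toward drift turns.
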(event `self.ReceiveBeginPlay`)

(event `InputAction|Accelerate`
  (params (Key :type "Key Structure"))
  (:`Pressed`
    (set `self.accelerate` true))
  (:`Released`
    (set `self.accelerate` false)))

(event `InputAction|LeftTurn`
  (params (Key :type "Key Structure"))
  (:`Pressed`
    (set `self.leftTurn` true)
    (set `self.turnDirection` -1.0))
  (:`Released`
    (set `self.leftTurn` false)
    (set `self.turnDirection` 0.0)))

(event `InputAction|RightTurn`
  (params (Key :type "Key Structure"))
  (:`Pressed`
    (set `self.rightTurn` true)
    (set `self.turnDirection` 1.0))
  (:`Released`
    (set `self.rightTurn` false)
    (set `self.turnDirection` 0.0)))

(event `self.ReceiveTick`
  (params (DeltaSeconds :type "Float (single-precision)"))
  (bind _springarm (`self.SpringArm`))
  (`|ExecutionSequence`
    (:`then_0`
      ;[1 1 1] Check if grounded
      (bind (_out_hit _return_value) (`self.LineTraceFromComponent` (`self.Car`) -60.0))
      (set `self.isGrounded` _return_value))
    (:`then_1`
      ;[1 1 1] Car Movement
      (if (and (`self.accelerate`) (< (`KismetMathLibrary.VSizeXY` (`self.GetVelocity`)) (`self.topSpeed`)))
        (`self.AccelerateCar`)
        (if (< (`KismetMathLibrary.VSizeXY` (`self.GetVelocity`)) (+ (`self.topSpeed`) (`self.strafeSpeed`)))
          (`self.StrafeCar` (`self.strafeDirection`)))
        (if (and (`self.isGrounded`) (!= (`self.turnDirection`) 0.0))
          (`self.TurnCar` (`self.turnDirection`))
          (if (and (`self.drift`) (not (`self.Boost`)))
            (`self.DriftCar`)
            (set `self.topSpeed` (`self.DriftTopSpeed`))
            (else
              (set `self.currentTurnForce` (`self.defaultTurnForce`))
              (if (and (`self.Boost`) (>= (`self.currentRad`) 1.0)) :!label _label
                (set `self.topSpeed` (`self.boostTopSpeed`))
                (set `self.currentRad` (- (`self.currentRad`) 1.0))
                (else
                  (set `self.topSpeed` (`self.driveTopSpeed`))))))
          (else
            (goto _label)))))
    (:`then_2`
      ;[1 1 1] Generate Stats
      (`self.GetCurrentSpeed`))
    (:`then_3`
      ;[1 1 1] Camera Movement
      (`CameraComponent.SetFieldOfView` (`self.Camera`) (+ (/ (`self.currentSpeed`) 100.0) 90.0))
      (if (and (or (`self.rightTurn`) (`self.leftTurn`)) (`self.drift`))
        (`self.DriftCameraAngle` (`self.turnDirection`))
        (else
          (`SceneComponent.K2_SetRelativeRotation` _springarm (`KismetMathLibrary.RLerp` (`SceneComponent.RelativeRotation` _springarm) (`KismetMathLibrary.MakeRotator` 0.0 -10.0) 0.1) false false))))))

(event `InputAction|Drift`
  (params (Key :type "Key Structure"))
  (:`Pressed`
    (set `self.drift` true))
  (:`Released`
    (set `self.drift` false)))

(event `InputAction|LeftStrafe`
  (params (Key :type "Key Structure"))
  (:`Pressed`
    (set `self.leftStrafe` true)
    (set `self.strafeDirection` -1))
  (:`Released`
    (set `self.leftStrafe` false)
    (set `self.strafeDirection` 0)))

(event `InputAction|RightStrafe`
  (params (Key :type "Key Structure"))
  (:`Pressed`
    (set `self.rightStrafe` true)
    (set `self.strafeDirection` 1))
  (:`Released`
    (set `self.rightStrafe` false)
    (set `self.strafeDirection` 0)))

(event `InputAction|Boost`
  (params (Key :type "Key Structure"))
  (:`Pressed`
    (set `self.Boost` true))
  (:`Released`
    (set `self.Boost` false)))

(fn `AccelerateCar`
  (bind (_returnvalue_x _returnvalue_y _returnvalue_z) (`KismetMathLibrary.BreakVector` (`self.GetVelocity`)))
  (bind (_returnvalue_x_2 _returnvalue_y_2) (`KismetMathLibrary.BreakVector` (* (`SceneComponent.GetForwardVector` (`self.Car`)) (`self.topSpeed`))))
  (bind (_returnvalue_x_3 _returnvalue_y_3) (`KismetMathLibrary.BreakVector` (`KismetMathLibrary.VLerp` (`KismetMathLibrary.MakeVector` _returnvalue_x _returnvalue_y _returnvalue_z) (`KismetMathLibrary.MakeVector` _returnvalue_x_2 _returnvalue_y_2) (`self.Acceleration`))))
  (`PrimitiveComponent.SetPhysicsLinearVelocity` (`self.Car`) (`KismetMathLibrary.MakeVector` _returnvalue_x_3 _returnvalue_y_3) true "None"))

(fn `DriftCameraAngle`
  (params (direction :type "Float (double-precision)"))
  (bind _springarm (`self.SpringArm`))
  (`SceneComponent.K2_SetRelativeRotation` _springarm (`KismetMathLibrary.RLerp` (`SceneComponent.RelativeRotation` _springarm) (`KismetMathLibrary.MakeRotator` 0.0 -10.0 (* direction -25.0)) 0.05) false false))

(fn `DriftCar`
  (set `self.currentTurnForce` (`KismetMathLibrary.Lerp` (`self.currentTurnForce`) (`self.driftForce`) 0.01))
  (if true
    (set `self.currentRad` (+ (`self.currentRad`) 1.0))))

(fn `GetCurrentSpeed`
  (bind _returnvalue (`PrimitiveComponent.GetPhysicsLinearVelocity` (`self.Car`) "None"))
  (set `self.currentSpeed` (`KismetMathLibrary.VSizeXY` _returnvalue)))

(fn `LineTraceFromComponent`
  (params (Component :type "SceneComponent Object Reference") (Length :type "Float (double-precision)"))
  (returns (`Out Hit` :type "HitResult Structure") (`Return Value` :type Boolean))
  (bind _returnvalue (`SceneComponent.K2_GetComponentLocation` Component))
  (bind (_outhit _returnvalue_2) (`KismetSystemLibrary.LineTraceSingleForObjects` :`Start` _returnvalue :`End` (+ _returnvalue (* (`KismetMathLibrary.GetUpVector` (`SceneComponent.K2_GetComponentRotation` Component)) Length)) :`ObjectTypes` (`self.Object Types`) :`DrawDebugType` "ForOneFrame"))
  (return _outhit _returnvalue_2))

(fn `StrafeCar`
  (params (direction :type Integer))
  (bind (_returnvalue_x _returnvalue_y) (`KismetMathLibrary.BreakVector` (* (`SceneComponent.GetRightVector` (`self.Car`)) (`self.strafeSpeed`) direction)))
  (`PrimitiveComponent.SetPhysicsLinearVelocity` (`self.Car`) (`KismetMathLibrary.MakeVector` _returnvalue_x _returnvalue_y) true "None"))

(fn `TurnCar`
  (params (direction :type "Float (double-precision)"))
  (`SceneComponent.K2_AddWorldRotation` (`self.Car`) (`KismetMathLibrary.MakeRotator` 0.0 0.0 (* (`self.currentTurnForce`) direction)) false false))

(fn `UserConstructionScript`)